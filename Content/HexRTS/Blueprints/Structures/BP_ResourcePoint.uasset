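; BP_ResourcePoint is a capturable resource point structure in the HexRTS game that reports its lifecycle to the RTS game mode.
; On BeginPlay it registers itself with RTSGameMode through ServerPointSpawned.
; When conquest is notified, it passes the conquering player's ID and its own resource ID to RTSGameMode's ServerPlayerCapturedResource, leaving capture handling to the game mode.
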(event EventBeginPlay
  (Default|ServerPointSpawned (.AsRTSGame%20Mode (Utilities|Casting|CastToRTSGameMode (Game|GetGameMode))) self))

(event EventNotifyServerConquest
  (Default|ServerPlayerCapturedResource (.AsRTSGame%20Mode (Utilities|Casting|CastToRTSGameMode (Game|GetGameMode))) (Variables|Default|GetConqueredID) (Variables|Default|GetID)))

(event EventTick
  (params (DeltaSeconds :type Float%20%28single-precision%29))
  (|CallParentFunction DeltaSeconds))

(fn ConstructionScript)