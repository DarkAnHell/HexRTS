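; BP_ObjectivePoint is a capturable objective structure for the HexRTS game, built on a parent class that supplies its begin play, tick and construction logic.
; When conquest is notified, it reports the conquering player's ID and its own ID to RTSGameMode as a captured resource.
; Debug strings print both IDs before that call.
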(event EventBeginPlay
  (|CallParentFunction))

(event EventTick
  (params (DeltaSeconds :type Float%20%28single-precision%29))
  (|CallParentFunction DeltaSeconds))

(event EventNotifyServerConquest
  (bind _id (Variables|Default|GetID))
  (bind _conqueredid (Variables|Default|GetConqueredID))
  (Development|PrintString "OBJECTIVE")
  (Development|PrintString (Utilities|String|ToString(Integer) _conqueredid))
  (Development|PrintString (Utilities|String|ToString(Integer) _id))
  (Default|ServerPlayerCapturedResource (.AsRTSGame%20Mode (Utilities|Casting|CastToRTSGameMode (Game|GetGameMode))) _conqueredid _id))

(fn ConstructionScript
  (|CallParentFunction))