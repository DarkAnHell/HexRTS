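; BP_Base is a player's base structure in HexRTS, whose destruction ends the match.
; On BeginPlay the server registers it with RTSGameMode, noted as the step that assigns its ID, and binds its damage handler.
; Damage is truncated to an integer and subtracted from HealthLeft.
; At zero or below, it increments ID and passes that modulo two to PlayerWon, crediting the opponent in a two-player match.
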(event Custom|OnTakeAnyDamage_Event_0
  (params (DamagedActor :type Actor%20Object%20Reference) (Damage :type Float%20%28single-precision%29) (DamageType :type Damage%20Type%20Object%20Reference) (InstigatedBy :type Controller%20Object%20Reference) (DamageCauser :type Actor%20Object%20Reference))
  ;[1 1 1] Take damage
  (Variables|Default|SethealthLeft (- (Variables|Default|GethealthLeft) (Math|Float|Truncate Damage)))
  (CallFunction|CheckHealth))

(event EventBeginPlay
  ;[1 1 1] Make server assign us an id
  (Networking|SwitchHasAuthority
    (:Authority
      (Default|ServerBaseSpawned (.AsRTSGame%20Mode (Utilities|Casting|CastToRTSGameMode (Game|GetGameMode))) self)
      ;[1 1 1] Take damage
      (EventDispatchers|AssignOnTakeAnyDamage (delegate Custom|OnTakeAnyDamage_Event_0)))))

(fn ConstructionScript
  (|CallParentFunction))

(fn CheckHealth
  (if (<= (Variables|Default|GethealthLeft) 0)
    (bind _result (Math|Integer|IncrementInt (Variables|Default|GetID))
      (:%20%20
        (Default|PlayerWon (.AsRTSGame%20Mode (Utilities|Casting|CastToRTSGameMode (Game|GetGameMode))) (Math|Integer|%(Integer) _result 2))))))