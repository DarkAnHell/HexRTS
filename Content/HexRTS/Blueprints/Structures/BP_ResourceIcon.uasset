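; BP_ResourceIcon is a Paper2D sprite icon for a resource, registered to appear on the minimap.
; On BeginPlay it finds the first BP_Minimap and adds itself to that scene capture's ShowOnlyActors list.
; The SetOwningPlayer event tints the sprite teal for player 0 or dark red for player 1.
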(event Custom|SetOwningPlayer
  (params (ID :type Integer))
  (switch int ID
    (:0
      (Sprite|SetSpriteColor (Variables|Default|GetPaperSprite) "(R=0.000000,G=0.505182,B=0.600000,A=1.000000)"))
    (:1
      (Sprite|SetSpriteColor (Variables|Default|GetPaperSprite) "(R=0.287500,G=0.014226,B=0.000000,A=1.000000)"))))

(event EventBeginPlay
  (bind _outactors (Actor|GetAllActorsOfClass "/Game/HexRTS/HUD/BP_Minimap.BP_Minimap_C"))
  (Utilities|Array|Add (Variables|/Script/Engine.SceneCaptureComponent|GetShowOnlyActors (Variables|/Script/Engine.SceneCapture2D|GetCaptureComponent2D (Utilities|Array|Get(acopy) _outactors))) self))

(event Collision|EventActorBeginOverlap
  (params (OtherActor :type Actor%20Object%20Reference)))

(fn ConstructionScript)