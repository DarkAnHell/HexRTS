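; Capturable map point that a player's units conquer by staying inside its area sphere for a set time.
; Server-side overlap events start, dispute or cancel a capture; rival units pause the countdown.
; Tick counts down locally to avoid replicating remaining time, while only the server commits the new owner.
; Capture then calls an empty NotifyServerConquest hook and recolors or updates the objective or resource icon's owner.
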(event OnComponentBeginOverlap(AreaSphere)
  (params (OverlappedComponent :type Primitive%20Component%20Object%20Reference) (OtherActor :type Actor%20Object%20Reference) (OtherComp :type Primitive%20Component%20Object%20Reference) (OtherBodyIndex :type Integer) (bFromSweep :type Boolean) (SweepResult :type Hit%20Result%20Structure%20%28by%20ref%29))
  ;[1 1 1] Start capturing point on server
  (Networking|SwitchHasAuthority
    (:Authority
      (if (and (< (Variables|conqueststate|GetisBeingConquered) 0) (!= (Variables|/Game/HexRTS/Blueprints/Units/BP_Unit.BP_Unit_C|GetPlayer (.AsBP%20Unit (Utilities|Casting|CastToBP_Unit OtherActor))) (Variables|conqueststate|GetConqueredID)))
        (Development|PrintString "BABY")
        ;;[1 1 1] Start conquering
        (bind _asbp_unit (Utilities|Casting|CastToBP_Unit OtherActor))
        (Variables|conqueststate|SetisBeingConquered (Variables|/Game/HexRTS/Blueprints/Units/BP_Unit.BP_Unit_C|GetPlayer _asbp_unit))
        (Variables|conqueststate|SetcurrentTimeToConquer (Variables|Config|GetTimeToConquer))
        (else
          (Development|PrintString "NICE TRY")
          ;;[1 1 1] Dispute point if different teams are near
          (bind _asbp_unit_2 (Utilities|Casting|CastToBP_Unit OtherActor))
          (if (!= (Variables|/Game/HexRTS/Blueprints/Units/BP_Unit.BP_Unit_C|GetPlayer _asbp_unit_2) (Variables|conqueststate|GetisBeingConquered))
            (Variables|conqueststate|SetisBeingDisputed true)))))))

(event OnComponentEndOverlap(AreaSphere)
  (params (OverlappedComponent :type Primitive%20Component%20Object%20Reference) (OtherActor :type Actor%20Object%20Reference) (OtherComp :type Primitive%20Component%20Object%20Reference) (OtherBodyIndex :type Integer))
  (bind _areasphere (Variables|Default|GetAreaSphere))
  (bind _overlappingactors (Collision|GetOverlappingActors _areasphere "/Game/HexRTS/Blueprints/Units/BP_Unit.BP_Unit_C" :!class /Script/Engine.PrimitiveComponent))
  ;[1 1 1] If a unit left and someone is capturing
  (Networking|SwitchHasAuthority
    (:Authority
      (if (>= (Variables|conqueststate|GetisBeingConquered) 0)
        ;[1 1 1] If no one else near, stop conquering
        (if (== (Utilities|Array|Length _overlappingactors) 0)
          (Variables|conqueststate|SetisBeingConquered -2)
          (Variables|conqueststate|SetcurrentTimeToConquer (Variables|Config|GetTimeToConquer))
          (else
            ;[1 1 1] Check if still contested
            (if (Variables|conqueststate|GetisBeingDisputed)
              (Variables|conqueststate|SetisstillDisputed false)
              (bind _array_element (Utilities|Array|ForEachLoopwithBreak _overlappingactors :!label _label)
                (:LoopBody
                  (bind _asbp_unit (Utilities|Casting|CastToBP_Unit _array_element))
                  (if (!= (Variables|/Game/HexRTS/Blueprints/Units/BP_Unit.BP_Unit_C|GetPlayer _asbp_unit) (Variables|conqueststate|GetisBeingConquered))
                    (Variables|conqueststate|SetisstillDisputed true)
                    (goto _label Break)))
                (:Completed
                  (if (not (Variables|conqueststate|GetisstillDisputed))
                    (Variables|conqueststate|SetisBeingDisputed false)))))))))))

(event Custom|UpdateIcon
  (bind _icon_ref (Variables|Default|GetIcon_ref))
  (bind _asbp_objective_icon (Utilities|Casting|CastToBP_ObjectiveIcon _icon_ref)
    (:then
      (Default|SetOwningPlayer _asbp_objective_icon (Variables|conqueststate|GetConqueredID)))
    (:CastFailed
      (bind _asbp_resource_icon (Utilities|Casting|CastToBP_ResourceIcon _icon_ref))
      (Default|SetOwningPlayer _asbp_resource_icon (Variables|conqueststate|GetConqueredID)))))

(event EventTick
  (params (DeltaSeconds :type Float%20%28single-precision%29))
  ;[1 1 1] Tick - Conquer a point
  (if (and (not (Variables|conqueststate|GetisBeingDisputed)) (>= (Variables|conqueststate|GetisBeingConquered) 0))
    (bind _output_get (Variables|conqueststate|SetcurrentTimeToConquer (- (Variables|conqueststate|GetcurrentTimeToConquer) DeltaSeconds)))
    ;;[1 1 1] Note how players calculate the time for themselfs as to not clog the network with updates on the time left, but the authoritative time on when a point is captured remains on the server
    (if (<= _output_get 0.0)
      (Networking|SwitchHasAuthority
        (:Authority
          (Variables|conqueststate|SetConqueredID (Variables|conqueststate|GetisBeingConquered))
          (Variables|conqueststate|SetisBeingConquered -2)
          (Variables|conqueststate|SetcurrentTimeToConquer (Variables|Config|GetTimeToConquer))
          (CallFunction|NotifyServerConquest)
          (CallFunction|UpdateIcon))))))

(fn ConstructionScript)

(fn IsConquered
  (return (>= (Variables|conqueststate|GetConqueredID) 0)))

(fn NotifyServerConquest)