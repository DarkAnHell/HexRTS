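; BP_MapPoint is a map point actor in the HexRTS game that can test line-of-sight connections to other points.
; On BeginPlay, the server registers it with RTSGameMode, which per the author's comment assigns it an id.
; CheckPathToPoint traces on Visibility to a given point, reporting connected if the hit is any BP_CapturablePoint, not necessarily the target.
; A trace with no hit prints an error and reports unconnected.
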(event EventBeginPlay
  ;[1 1 1] Make server assign us an id
  (Networking|SwitchHasAuthority
    (:Authority
      (Default|ServerPointSpawned (.AsRTSGame%20Mode (Utilities|Casting|CastToRTSGameMode (Game|GetGameMode))) self))))

(event EventTick
  (params (DeltaSeconds :type Float%20%28single-precision%29)))

(fn ConstructionScript)

(fn CheckPathtoPoint
  (params (point :type BP%20Capturable%20Point%20Object%20Reference))
  ;[1 1 1] Raycast
  (bind (_outhit _returnvalue) (Collision|LineTraceByChannel (Transformation|GetActorLocation) (Transformation|GetActorLocation point) "TraceTypeQuery1" false 0 "ForOneFrame"))
  (if _returnvalue
    ;[1 1 1] Check if we hit a point
    (Utilities|Casting|CastToBP_CapturablePoint (.HitActor (Collision|BreakHitResult _outhit))
      (:then
        (LocalVariables|SetisConnected true))
      (:CastFailed
        (LocalVariables|SetisConnected false :!label _label)))
    (else
      ;[1 1 1] No hit
      (Development|PrintString "ERROR: No point detected by raycast" true true "(R=1.000000,G=0.059196,B=0.000000,A=1.000000)" 2e+01)
      (goto _label)))
  (return (LocalVariables|GetisConnected)))