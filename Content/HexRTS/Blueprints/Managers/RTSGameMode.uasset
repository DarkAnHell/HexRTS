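; Server game mode for a two-player RTS: spawns bases, objective and resource points at hardcoded locations, plus player pawns and minimap icons.
; Capture events record owners in RTSGameState, adjusting resources or income rates and the leading player.
; Looping timers pay income and add points for the leader's objectives toward victory, resetting when the lead changes.
; Tick alternately creates units at each base; the win only prints.
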(event Custom|Server_ObjectiveSpawned
  (params (Objective :type BP%20Objective%20Point%20Object%20Reference))
  (bind _returnvalue (Transformation|GetActorLocation Objective))
  (bind _objectivecounter (Variables|Default|GetobjectiveCounter))
  (bind (_x _y) (Math|Vector|BreakVector _returnvalue))
  ;[1 1 1] Assign ID, ICON to resource or objective points
  (bind _returnvalue_2 (Game|SpawnActorfromClass "/Game/HexRTS/Blueprints/Structures/BP_ObjectiveIcon.BP_ObjectiveIcon_C" (Math|Transform|MakeTransform (Math|Vector|MakeVector _x _y 2e+04)) "Undefined" 0 Objective 0))
  (Variables|/Game/HexRTS/Blueprints/Structures/BP_CapturablePoint.BP_CapturablePoint_C|SetIcon_ref Objective _returnvalue_2)
  (Development|PrintString (Utilities|String|ToString(Integer) _objectivecounter))
  ;;[1 1 1] Set ID
  (Variables|/Game/HexRTS/Blueprints/Structures/BP_MapPoint.BP_MapPoint_C|SetID Objective _objectivecounter)
  (Math|Integer|IncrementInt _objectivecounter
    (:%20%20
      ;;[1 1 1] Configure conquer time
      (Variables|/Game/HexRTS/Blueprints/Structures/BP_CapturablePoint.BP_CapturablePoint_C|SetTimeToConquer Objective (Variables|Objectives|GetTimeToConquerObjective)))))

(event Custom|Server_createUnit
  (params (position :type Vector) (playerID :type Integer))
  ;[1 1 1] Unit Creation
  (bind _returnvalue (AI|SpawnAIFromClass "/Game/HexRTS/Blueprints/Units/BP_Unit.BP_Unit_C" "/Game/HexRTS/Blueprints/Units/AI/BHT_Unit.BHT_Unit" position "0, 0, 0" true))
  (Variables|/Game/HexRTS/Blueprints/Units/BP_Unit.BP_Unit_C|SetPlayer (.AsBP%20Unit (Utilities|Casting|CastToBP_Unit _returnvalue)) playerID)
  (bind _returnvalue_2 (Game|SpawnActorfromClass "/Game/HexRTS/Blueprints/Units/BP_UnitFollow.BP_UnitFollow_C" (Math|Transform|MakeTransform (Math|Vector|MakeVector (.X (Math|Vector|BreakVector (Transformation|GetActorLocation (.AsBP%20Unit (Utilities|Casting|CastToBP_Unit _returnvalue))))) (.Y (Math|Vector|BreakVector (Transformation|GetActorLocation (.AsBP%20Unit (Utilities|Casting|CastToBP_Unit _returnvalue))))) 2e+04)) "Undefined" 0 (.AsBP%20Unit (Utilities|Casting|CastToBP_Unit _returnvalue)) 0))
  (Variables|/Game/HexRTS/Blueprints/Units/BP_Unit.BP_Unit_C|SetminimapIcon_ref (.AsBP%20Unit (Utilities|Casting|CastToBP_Unit _returnvalue)) _returnvalue_2))

(event Custom|Server_PlayerCapturedResource
  (params (PlayerID :type Integer) (ResourceID :type Integer))
  (bind _gamestateref (Variables|Default|GetGameStateRef))
  (bind _gamestateref_2 (Variables|Default|GetGameStateRef))
  (bind _gamestateref_3 (Variables|Default|GetGameStateRef))
  (bind _resourceobjectives (Variables|/Game/HexRTS/Blueprints/Managers/RTSGameState.RTSGameState_C|GetResourceObjectives _gamestateref))
  (bind _resourcesperplayer (Variables|/Game/HexRTS/Blueprints/Managers/RTSGameState.RTSGameState_C|GetresourcesPerPlayer _gamestateref_2))
  (bind _resourcesperplayer_2 (Variables|/Game/HexRTS/Blueprints/Managers/RTSGameState.RTSGameState_C|GetresourcesPerPlayer _gamestateref_3))
  (bind (_value _returnvalue) (Utilities|Map|Find _resourcesperplayer_2 PlayerID))
  (bind _output (Utilities|Array|Get(acopy) _resourceobjectives ResourceID))
  (bind _value_2 (Utilities|Map|Find _resourcesperplayer _output))
  ;[0.7047 1 0.6537] Update resources to mark one as captured
  ;[1 1 1] Can't capture more than once
  (if (!= (Utilities|Array|Get(acopy) _resourceobjectives ResourceID) PlayerID)
    ;[1 1 1] Reduce the other player's rate if there was any
    (if (!= _output -1)
      (Variables|/Game/HexRTS/Blueprints/Managers/RTSPlayerState.RTSPlayerState_C|SetCurrentResourcesRate _value_2 (- (Variables|/Game/HexRTS/Blueprints/Managers/RTSPlayerState.RTSPlayerState_C|GetCurrentResourcesRate _value_2) (Variables|Resources|GetResourcesDOGEPerCapture))))
    ;[1 1 1] Update resources array
    (Utilities|Array|SetArrayElem (Variables|/Game/HexRTS/Blueprints/Managers/RTSGameState.RTSGameState_C|GetResourceObjectives (Variables|Default|GetGameStateRef)) ResourceID PlayerID true)
    ;[1 1 1] Update Player rate
    (if _returnvalue
      (Variables|/Game/HexRTS/Blueprints/Managers/RTSPlayerState.RTSPlayerState_C|SetCurrentResourcesRate _value (+ (Variables|Resources|GetResourcesDOGEPerCapture) (Variables|/Game/HexRTS/Blueprints/Managers/RTSPlayerState.RTSPlayerState_C|GetCurrentResourcesRate _value))))))

(event Custom|Server_PlayerCapturedObjective
  (params (PlayerID :type Integer) (ObjectiveID :type Integer))
  (bind _returnvalue (Game|GetGameState))
  (bind _asrtsgame_state (Utilities|Casting|CastToRTSGameState _returnvalue))
  (bind _objectives (Variables|/Game/HexRTS/Blueprints/Managers/RTSGameState.RTSGameState_C|GetObjectives _asrtsgame_state))
  (bind _resourcesperplayer (Variables|/Game/HexRTS/Blueprints/Managers/RTSGameState.RTSGameState_C|GetresourcesPerPlayer _asrtsgame_state))
  (bind _value (Utilities|Map|Find _resourcesperplayer PlayerID))
  ;[0.74 1 0.4999] Update Objective capture
  (Development|PrintString (Utilities|String|Append "CAPTURED " (Utilities|String|ToString(Integer) ObjectiveID)))
  ;[1 1 1] Can't capture more than once
  (if (!= (Utilities|Array|Get(acopy) _objectives ObjectiveID) PlayerID)
    ;[1 1 1] Update Objectives
    (Utilities|Array|SetArrayElem _objectives ObjectiveID PlayerID true)
    ;[1 1 1] Update Resources
    (Variables|/Game/HexRTS/Blueprints/Managers/RTSPlayerState.RTSPlayerState_C|SetCurrentResources _value (+ (Variables|/Game/HexRTS/Blueprints/Managers/RTSPlayerState.RTSPlayerState_C|GetCurrentResources _value) (Variables|Resources|GetResourcesOnObjectiveCapture)))
    (CallFunction|RecalculateObjectives)))

(event Custom|Server_ResourceSpawned
  (params (resource :type BP%20Resource%20Point%20Object%20Reference))
  (bind _returnvalue (Transformation|GetActorLocation resource))
  (bind _resourcecounter (Variables|Default|GetresourceCounter))
  (bind (_x _y) (Math|Vector|BreakVector _returnvalue))
  ;[1 1 1] Assign ID, ICON to resource or objective points
  (bind _returnvalue_2 (Game|SpawnActorfromClass "/Game/HexRTS/Blueprints/Structures/BP_ResourceIcon.BP_ResourceIcon_C" (Math|Transform|MakeTransform (Math|Vector|MakeVector _x _y 2e+04)) "Undefined" 0 resource 0))
  (Variables|/Game/HexRTS/Blueprints/Structures/BP_CapturablePoint.BP_CapturablePoint_C|SetIcon_ref resource _returnvalue_2)
  ;;[1 1 1] Set ID
  (Variables|/Game/HexRTS/Blueprints/Structures/BP_MapPoint.BP_MapPoint_C|SetID resource _resourcecounter)
  (Math|Integer|IncrementInt _resourcecounter
    (:%20%20
      ;;[1 1 1] Configure conquer time
      (Variables|/Game/HexRTS/Blueprints/Structures/BP_CapturablePoint.BP_CapturablePoint_C|SetTimeToConquer resource (Variables|Resources|GetTimeToConquerResource)))))

(event Custom|Server_BaseSpawned
  (params (Base :type BP%20Base%20Object%20Reference))
  (Variables|/Game/HexRTS/Blueprints/Structures/BP_Base.BP_Base_C|SethealthLeft Base (Variables|Bases|GetBaseInitialHealth)))

(event EventTick
  (params (DeltaSeconds :type Float%20%28single-precision%29))
  (bind _outactors (Actor|GetAllActorsOfClass "/Game/HexRTS/Blueprints/Structures/BP_Base.BP_Base_C"))
  (Utilities|FlowControl|FlipFlop
    (:A
      (CallFunction|ServerCreateUnit (Math|Vector|MakeVector (+ (.X (Math|Vector|BreakVector (Transformation|GetActorLocation (Utilities|Array|Get(acopy) _outactors)))) -5e+02) (+ (.Y (Math|Vector|BreakVector (Transformation|GetActorLocation (Utilities|Array|Get(acopy) _outactors)))) -5e+02) (.Z (Math|Vector|BreakVector (Transformation|GetActorLocation (Utilities|Array|Get(acopy) _outactors))))) (Variables|/Game/HexRTS/Blueprints/Structures/BP_MapPoint.BP_MapPoint_C|GetID (Utilities|Array|Get(acopy) _outactors))))
    (:B
      (CallFunction|ServerCreateUnit (Math|Vector|MakeVector (+ (.X (Math|Vector|BreakVector (Transformation|GetActorLocation (Utilities|Array|Get(acopy) _outactors 1)))) -5e+02) (+ (.Y (Math|Vector|BreakVector (Transformation|GetActorLocation (Utilities|Array|Get(acopy) _outactors 1)))) -5e+02) (.Z (Math|Vector|BreakVector (Transformation|GetActorLocation (Utilities|Array|Get(acopy) _outactors 1))))) (Variables|/Game/HexRTS/Blueprints/Structures/BP_MapPoint.BP_MapPoint_C|GetID (Utilities|Array|Get(acopy) _outactors 1))))))

(event EventBeginPlay
  (Variables|Default|SetGameStateRef (.AsRTSGame%20State (Utilities|Casting|CastToRTSGameState (Game|GetGameState))))
  ;[1 1 1] Set timer for objective checking
  (Utilities|Time|SetTimerbyFunctionName 0 "PeriodicRecalculatePoints" (Variables|Objectives|GetObjectiveTick) true)
  ;[1 1 1] Timer for resources
  (Utilities|Time|SetTimerbyFunctionName 0 "PeriodicGiveResources" (Variables|Resources|GetResourcesTick) true)
  ;[1 1 1] Init bases
  (CallFunction|PlaceBases)
  ;[1 1 1] Initialize Objectives
  (for _index (range 0 (- (Variables|Objectives|GetObjectiveNumber) 1))
    (Utilities|Array|Add (Variables|/Game/HexRTS/Blueprints/Managers/RTSGameState.RTSGameState_C|GetObjectives (Variables|Default|GetGameStateRef)) -1))
  (CallFunction|PlaceObjectives)
  (CallFunction|PlaceResources)
  ;[1 1 1] Init Resources
  (for _index_2 (range 0 (- (Variables|Default|GetresourceCounter) 1))
    (Utilities|Array|Add (Variables|/Game/HexRTS/Blueprints/Managers/RTSGameState.RTSGameState_C|GetResourceObjectives (Variables|Default|GetGameStateRef)) -1)))

(event EventPostLogin
  (params (NewPlayer :type Player%20Controller%20Object%20Reference))
  (bind _playercounter (Variables|Default|Getplayercounter))
  ;[1 1 1] On post login
  ;[0.5094 0.9701 1] Spawn player main map
  (bind _returnvalue (Game|SpawnActorfromClass "/Game/HexRTS/Blueprints/Characters/BP_Player.BP_Player_C" (Math|Transform|MakeTransform "0, 0, 0") "AlwaysSpawn" NewPlayer 0))
  (Pawn|Possess NewPlayer _returnvalue)
  ;[1 1 1] Assign ID to player
  (bind _asrtsplayer_controller (Utilities|Casting|CastToRTSPlayerController NewPlayer))
  (Variables|/Game/HexRTS/Blueprints/Managers/RTSPlayerController.RTSPlayerController_C|SetID _asrtsplayer_controller _playercounter)
  (Math|Integer|IncrementInt _playercounter))

(fn ConstructionScript)

(fn PlayerWon
  (params (playerID :type Integer))
  ;[1 1 1] TODO: Print win screen , freeze time
  (Development|PrintString (Utilities|String|Append "PLAYER WON:" (Utilities|String|ToString(Integer) playerID))))

(fn CheckifPlayerWon
  (bind _returnvalue (Game|GetGameState))
  (bind (_asrtsgame_state _bsuccess) (Utilities|Casting|CastToRTSGameState _returnvalue))
  ;[1 1 1] Check if someone won by objectives
  (if _bsuccess
    (if (>= (Variables|/Game/HexRTS/Blueprints/Managers/RTSGameState.RTSGameState_C|GetPoints _asrtsgame_state) (Variables|Objectives|GetObjectivePointsToWin))
      ;[1 1 1] Player WON
      (CallFunction|PlayerWon (Variables|/Game/HexRTS/Blueprints/Managers/RTSGameState.RTSGameState_C|GetplayerIDWinning _asrtsgame_state)))
    (else
      (Development|PrintString "ERROR while casting to gamestate"))))

(fn PeriodicGiveResources
  ;[1 1 1] Increment resources by rate
  (bind _values (Utilities|Map|Values (Variables|/Game/HexRTS/Blueprints/Managers/RTSGameState.RTSGameState_C|GetresourcesPerPlayer (Variables|Default|GetGameStateRef))))
  (for _array_element _values
    (Variables|/Game/HexRTS/Blueprints/Managers/RTSPlayerState.RTSPlayerState_C|SetCurrentResources _array_element (+ (Variables|/Game/HexRTS/Blueprints/Managers/RTSPlayerState.RTSPlayerState_C|GetCurrentResourcesRate _array_element) (Variables|/Game/HexRTS/Blueprints/Managers/RTSPlayerState.RTSPlayerState_C|GetCurrentResources _array_element)))))

(fn PeriodicRecalculatePoints
  (bind _gamestateref (Variables|Default|GetGameStateRef))
  ;[1 1 1] Reset counter
  (LocalVariables|SetObjectivesCapturedByWinningPlayer 0)
  ;[1 1 1] calculate points for player
  (for _array_element (Variables|/Game/HexRTS/Blueprints/Managers/RTSGameState.RTSGameState_C|GetObjectives _gamestateref)
    (if (== _array_element (Variables|/Game/HexRTS/Blueprints/Managers/RTSGameState.RTSGameState_C|GetplayerIDWinning _gamestateref))
      (bind _result (Math|Integer|IncrementInt (LocalVariables|GetObjectivesCapturedByWinningPlayer))
        (:%20%20
          (LocalVariables|SetObjectivesCapturedByWinningPlayer _result)))))
  ;[1 1 1] Update points
  (bind _output_get (Variables|/Game/HexRTS/Blueprints/Managers/RTSGameState.RTSGameState_C|SetPoints _gamestateref (+ (Variables|/Game/HexRTS/Blueprints/Managers/RTSGameState.RTSGameState_C|GetPoints _gamestateref) (* (LocalVariables|GetObjectivesCapturedByWinningPlayer) (Variables|Objectives|GetObjectivePointsPerCaptured)))))
  ;[1 1 1] Update Bar
  (Variables|/Game/HexRTS/Blueprints/Managers/RTSGameState.RTSGameState_C|SetPercentageOfBar _gamestateref (/ (Math|Conversions|ToFloat(Integer) _output_get) (Math|Conversions|ToFloat(Integer) (Variables|Objectives|GetObjectivePointsToWin))))
  ;[1 1 1] Check if someone won
  (CallFunction|CheckifPlayerWon))

(fn RecalculateObjectives
  (bind _gamestateref (Variables|Default|GetGameStateRef))
  ;[1 1 1] Reset local count
  (LocalVariables|SetPointsPlayer 0)
  ;[1 1 1] Count who is winning, by adding or subtracting points depending on which player has it.  Hardcoded players 0 and 1
  (for _array_element (Variables|/Game/HexRTS/Blueprints/Managers/RTSGameState.RTSGameState_C|GetObjectives (Variables|Default|GetGameStateRef))
    (if (== _array_element 0)
      (Math|Integer|IncrementInt (LocalVariables|GetPointsPlayer))
      (elif (== _array_element 1)
        (Math|Integer|DecrementInt (LocalVariables|GetPointsPlayer)))))
  ;[1 1 1] Check who is winning, reset points if the winner changed. Hardcoded players as 0 and 1
  (if (> (LocalVariables|GetPointsPlayer) 0)
    (if (!= (Variables|/Game/HexRTS/Blueprints/Managers/RTSGameState.RTSGameState_C|GetplayerIDWinning _gamestateref) 0)
      (Variables|/Game/HexRTS/Blueprints/Managers/RTSGameState.RTSGameState_C|SetplayerIDWinning _gamestateref 0)
      (Variables|/Game/HexRTS/Blueprints/Managers/RTSGameState.RTSGameState_C|SetPoints _gamestateref 0 :!label _label))
    (elif (< (LocalVariables|GetPointsPlayer) 0)
      (if (!= (Variables|/Game/HexRTS/Blueprints/Managers/RTSGameState.RTSGameState_C|GetplayerIDWinning _gamestateref) 1)
        (Variables|/Game/HexRTS/Blueprints/Managers/RTSGameState.RTSGameState_C|SetplayerIDWinning _gamestateref 1)
        (goto _label))
      (else
        (Variables|/Game/HexRTS/Blueprints/Managers/RTSGameState.RTSGameState_C|SetplayerIDWinning _gamestateref -2)
        (goto _label)))))

(fn PlaceObjectives
  (Game|SpawnActorfromClass "/Game/HexRTS/Blueprints/Structures/BP_ObjectivePoint.BP_ObjectivePoint_C" (Math|Transform|MakeTransform "5399.000000,5671.000000,60.000000") "Undefined" 0 0)
  (Game|SpawnActorfromClass "/Game/HexRTS/Blueprints/Structures/BP_ObjectivePoint.BP_ObjectivePoint_C" (Math|Transform|MakeTransform "5632.000000,18162.000000,60.000000") "Undefined" 0 0)
  (Game|SpawnActorfromClass "/Game/HexRTS/Blueprints/Structures/BP_ObjectivePoint.BP_ObjectivePoint_C" (Math|Transform|MakeTransform "16185.000000,25378.000000,50.000000") "Undefined" 0 0)
  (Game|SpawnActorfromClass "/Game/HexRTS/Blueprints/Structures/BP_ObjectivePoint.BP_ObjectivePoint_C" (Math|Transform|MakeTransform "30242.000000,30732.000000,50.000000") "Undefined" 0 0)
  (Game|SpawnActorfromClass "/Game/HexRTS/Blueprints/Structures/BP_ObjectivePoint.BP_ObjectivePoint_C" (Math|Transform|MakeTransform "31680.000000,40168.000000,50.000000") "Undefined" 0 0))

(fn PlaceResources
  (Game|SpawnActorfromClass "/Game/HexRTS/Blueprints/Structures/BP_ResourcePoint.BP_ResourcePoint_C" (Math|Transform|MakeTransform "24600.000000,42805.000000,51.000000") "Undefined" 0 0)
  (Game|SpawnActorfromClass "/Game/HexRTS/Blueprints/Structures/BP_ResourcePoint.BP_ResourcePoint_C" (Math|Transform|MakeTransform "11996.000000,6849.000000,32.000000") "Undefined" 0 0)
  (Game|SpawnActorfromClass "/Game/HexRTS/Blueprints/Structures/BP_ResourcePoint.BP_ResourcePoint_C" (Math|Transform|MakeTransform "28915.000000,7419.000000,308.000000") "Undefined" 0 0)
  (Game|SpawnActorfromClass "/Game/HexRTS/Blueprints/Structures/BP_ResourcePoint.BP_ResourcePoint_C" (Math|Transform|MakeTransform "19548.000000,16238.000000,222.000000") "Undefined" 0 0)
  (Game|SpawnActorfromClass "/Game/HexRTS/Blueprints/Structures/BP_ResourcePoint.BP_ResourcePoint_C" (Math|Transform|MakeTransform "8644.000000,16144.000000,102.000000") "Undefined" 0 0)
  (Game|SpawnActorfromClass "/Game/HexRTS/Blueprints/Structures/BP_ResourcePoint.BP_ResourcePoint_C" (Math|Transform|MakeTransform "6949.000000,40796.000000,11.000000") "Undefined" 0 0)
  (Game|SpawnActorfromClass "/Game/HexRTS/Blueprints/Structures/BP_ResourcePoint.BP_ResourcePoint_C" (Math|Transform|MakeTransform "21468.000000,44575.000000,1258.000000") "Undefined" 0 0)
  (Game|SpawnActorfromClass "/Game/HexRTS/Blueprints/Structures/BP_ResourcePoint.BP_ResourcePoint_C" (Math|Transform|MakeTransform "14642.000000,98067.000000,-183.000000") "Undefined" 0 0)
  (Game|SpawnActorfromClass "/Game/HexRTS/Blueprints/Structures/BP_ResourcePoint.BP_ResourcePoint_C" (Math|Transform|MakeTransform "32523.000000,31519.000000,30.000000") "Undefined" 0 0))

(fn PlaceBases
  (bind _returnvalue (Game|SpawnActorfromClass "/Game/HexRTS/Blueprints/Structures/BP_Base.BP_Base_C" (Math|Transform|MakeTransform "19658.000000,44335.000000,1590.000000" "0,180.000000,0.000000") "Undefined" 0 0))
  (Variables|/Game/HexRTS/Blueprints/Structures/BP_MapPoint.BP_MapPoint_C|SetID _returnvalue 0)
  (bind _returnvalue_2 (Game|SpawnActorfromClass "/Game/HexRTS/Blueprints/Structures/BP_Base.BP_Base_C" (Math|Transform|MakeTransform "18730.000000,3352.000000,1353.000000") "Undefined" 0 0))
  (Variables|/Game/HexRTS/Blueprints/Structures/BP_MapPoint.BP_MapPoint_C|SetID _returnvalue_2 1))

(fn PeriodicSpawnUnits)