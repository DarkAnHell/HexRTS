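; RTS game state that tracks objective and resource-point ownership, the leading player's score and per-player resources.
; On authority, BeginPlay sizes ownership arrays from RTSGameMode settings and starts looping timers for scoring and income.
; Captures update ownership, granting resources for objectives or shifting income rates for resource points.
; The objective majority, hardcoded for players 0 and 1, sets the leader, resetting points on change or tie; scoring ticks trigger GameMode's win check.
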(event Custom|Server_ObjectiveCapturedResources
  (params (playerID :type Integer) (objectiveID :type Integer))
  (bind _resourcesperplayer (Variables|Default|GetresourcesPerPlayer))
  (bind _value (Utilities|Map|Find _resourcesperplayer playerID))
  ;[1 1 1] Captured objective
  ;[1 1 1] Update Objectives
  (Utilities|Array|SetArrayElem (Variables|Default|GetObjectives) objectiveID playerID true)
  ;[1 1 1] Update Resources
  (Variables|/Game/HexRTS/Blueprints/Managers/RTSPlayerState.RTSPlayerState_C|SetCurrentResources _value (+ (Variables|/Game/HexRTS/Blueprints/Managers/RTSPlayerState.RTSPlayerState_C|GetCurrentResources _value) (Variables|/Game/HexRTS/Blueprints/Managers/RTSGameMode.RTSGameMode_C|GetResourcesOnObjectiveCapture (.AsRTSGame%20Mode (Utilities|Casting|CastToRTSGameMode (Game|GetGameMode))))))
  ;[1 1 1] Recalculate objectives
  (CallFunction|RecalculateObjectives))

(event Custom|Server_ResourceCaptured
  (params (PlayerID :type Integer) (ResourceID :type Integer))
  (bind _resourcesperplayer (Variables|Default|GetresourcesPerPlayer))
  (bind _resourceobjectives (Variables|Default|GetResourceObjectives))
  (bind _resourcesperplayer_2 (Variables|Default|GetresourcesPerPlayer))
  (bind (_value _returnvalue) (Utilities|Map|Find _resourcesperplayer_2 PlayerID))
  (bind _output (Utilities|Array|Get(acopy) _resourceobjectives ResourceID))
  (bind _value_2 (Utilities|Map|Find _resourcesperplayer _output))
  ;[1 1 1] Reduce the other player's rate if there was any
  (if (!= _output -1)
    (Variables|/Game/HexRTS/Blueprints/Managers/RTSPlayerState.RTSPlayerState_C|SetCurrentResourcesRate _value_2 (- (Variables|/Game/HexRTS/Blueprints/Managers/RTSPlayerState.RTSPlayerState_C|GetCurrentResourcesRate _value_2) (Variables|/Game/HexRTS/Blueprints/Managers/RTSGameMode.RTSGameMode_C|GetResourcesDOGEPerCapture (.AsRTSGame%20Mode (Utilities|Casting|CastToRTSGameMode (Game|GetGameMode)))))))
  ;[1 1 1] Update resources array
  (Utilities|Array|SetArrayElem (Variables|Default|GetResourceObjectives) ResourceID PlayerID true)
  ;[1 1 1] Update Player rate
  (if _returnvalue
    (Variables|/Game/HexRTS/Blueprints/Managers/RTSPlayerState.RTSPlayerState_C|SetCurrentResourcesRate _value (+ (Variables|/Game/HexRTS/Blueprints/Managers/RTSGameMode.RTSGameMode_C|GetResourcesDOGEPerCapture (.AsRTSGame%20Mode (Utilities|Casting|CastToRTSGameMode (Game|GetGameMode)))) (Variables|/Game/HexRTS/Blueprints/Managers/RTSPlayerState.RTSPlayerState_C|GetCurrentResourcesRate _value)))
    (else
      (Development|PrintString (Utilities|String|Append "ERROR: No player on map with that id ->" (Utilities|String|ToString(Integer) PlayerID)) true true "(R=1.000000,G=0.059606,B=0.000000,A=1.000000)" 5.0))))

(event EventBeginPlay
  (bind _returnvalue (Game|GetGameMode))
  (bind _asrtsgame_mode (Utilities|Casting|CastToRTSGameMode _returnvalue))
  ;[1 1 1] Begin play
  (Networking|SwitchHasAuthority
    (:Authority
      ;[1 1 1] Set timer for objective checking
      (Utilities|Time|SetTimerbyFunctionName 0 "PeriodicRecalculatePoints" (Variables|/Game/HexRTS/Blueprints/Managers/RTSGameMode.RTSGameMode_C|GetObjectiveTick _asrtsgame_mode) true)
      ;[1 1 1] Timer for resources
      (Utilities|Time|SetTimerbyFunctionName 0 "PeriodicGiveResources" (Variables|/Game/HexRTS/Blueprints/Managers/RTSGameMode.RTSGameMode_C|GetResourcesTick (.AsRTSGame%20Mode (Utilities|Casting|CastToRTSGameMode (Game|GetGameMode)))) true)
      ;[1 1 1] Initialize Objectives
      (for _index (range 0 (- (Variables|/Game/HexRTS/Blueprints/Managers/RTSGameMode.RTSGameMode_C|GetObjectiveNumber _asrtsgame_mode) 1))
        (Utilities|Array|Add (Variables|Default|GetObjectives) -1))
      ;[1 1 1] Init Resources
      (for _index_2 (range 0 (- (Variables|/Game/HexRTS/Blueprints/Managers/RTSGameMode.RTSGameMode_C|GetResourcesNumber _asrtsgame_mode) 1))
        (Utilities|Array|Add (Variables|Default|GetResourceObjectives) -1)))))

(fn ConstructionScript)

(fn RecalculateObjectives
  (Networking|SwitchHasAuthority
    (:Authority
      ;[1 1 1] Reset local count
      (LocalVariables|SetpointsPlayer 0)
      ;[1 1 1] Count who is winning, by adding or subtracting points depending on which player has it.  Hardcoded players 1 and 2
      (for _array_element (Variables|Default|GetObjectives)
        (Development|PrintString (Utilities|String|ToString(Integer) _array_element))
        (if (== _array_element 0)
          (Math|Integer|IncrementInt (LocalVariables|GetpointsPlayer)
            (:%20%20
              (LocalVariables|SetpointsPlayer (stale _result) :!label _label)))
          (elif (== _array_element 1)
            (bind _result (Math|Integer|DecrementInt (LocalVariables|GetpointsPlayer))
              (:%20%20
                (goto _label))))))
      ;[1 1 1] Check who is winning, reset points if the winner changed. Hardcoded players as 1 and 2
      (if (> (LocalVariables|GetpointsPlayer) 0)
        (if (!= (Variables|Default|GetplayerIDWinning) 0)
          (Variables|Default|SetplayerIDWinning 0)
          (Variables|Default|SetPoints 0 :!label _label_2))
        (elif (< (LocalVariables|GetpointsPlayer) 0)
          (if (!= (Variables|Default|GetplayerIDWinning) 1)
            (Variables|Default|SetplayerIDWinning 1)
            (goto _label_2))
          (else
            (Variables|Default|SetplayerIDWinning -2)
            (goto _label_2)))))))

(fn PeriodicRecalculatePoints
  (bind _returnvalue (Game|GetGameMode))
  (bind _asrtsgame_mode (Utilities|Casting|CastToRTSGameMode _returnvalue))
  (Networking|SwitchHasAuthority
    (:Authority
      ;[1 1 1] DEBUG
      (Development|PrintString (Utilities|String|Append "Winning:" (Utilities|String|ToString(Integer) (Variables|Default|GetplayerIDWinning))))
      (for (_array_element _array_index) (Variables|Default|GetObjectives)
        (Development|PrintString (Utilities|String|Append (Utilities|String|ToString(Integer) _array_index) "->" (Utilities|String|ToString(Integer) _array_element))))
      ;[1 1 1] Reset counter
      (LocalVariables|SetObjectivesCapturedByWinningPlayer 0)
      ;[1 1 1] calculate points for player
      (for _array_element_2 (Variables|Default|GetObjectives)
        (if (== _array_element_2 (Variables|Default|GetplayerIDWinning))
          (bind _result (Math|Integer|IncrementInt (LocalVariables|GetObjectivesCapturedByWinningPlayer))
            (:%20%20
              (LocalVariables|SetObjectivesCapturedByWinningPlayer _result)))))
      ;[1 1 1] Update points
      (bind _output_get (Variables|Default|SetPoints (+ (Variables|Default|GetPoints) (* (LocalVariables|GetObjectivesCapturedByWinningPlayer) (Variables|/Game/HexRTS/Blueprints/Managers/RTSGameMode.RTSGameMode_C|GetObjectivePointsPerCaptured _asrtsgame_mode)))))
      ;[1 1 1] Check if someone won
      (Default|CheckifPlayerWon _asrtsgame_mode)
      ;[1 1 1] DEBUG
      (Development|PrintString (Utilities|String|Append "Winning Points:" (Utilities|String|ToString(Integer) _output_get))))))

(fn PeriodicGiveResources
  ;[1 1 1] Increment resources by rate
  (bind _values (Utilities|Map|Values (Variables|Default|GetresourcesPerPlayer)))
  (for _array_element _values
    (Variables|/Game/HexRTS/Blueprints/Managers/RTSPlayerState.RTSPlayerState_C|SetCurrentResources _array_element (+ (Variables|/Game/HexRTS/Blueprints/Managers/RTSPlayerState.RTSPlayerState_C|GetCurrentResourcesRate _array_element) (Variables|/Game/HexRTS/Blueprints/Managers/RTSPlayerState.RTSPlayerState_C|GetCurrentResources _array_element)))))