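; Player state for the hex RTS that holds a player's current resource rate.
; On BeginPlay, only with authority, it seeds that rate from the default resources defined on the RTS game mode.
; It then registers itself in the game state's per-player resources map, using the map's current length as its key.
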(event EventBeginPlay
  (bind _returnvalue (Game|GetGameMode))
  (bind _returnvalue_2 (Game|GetGameState))
  (bind (_asrtsgame_mode _bsuccess) (Utilities|Casting|CastToRTSGameMode _returnvalue))
  (bind _asrtsgame_state (Utilities|Casting|CastToRTSGameState _returnvalue_2))
  (bind _resourcesperplayer (Variables|/Game/HexRTS/Blueprints/Managers/RTSGameState.RTSGameState_C|GetresourcesPerPlayer _asrtsgame_state))
  ;[1 1 1] Set default rate
  (Networking|SwitchHasAuthority
    (:Authority
      (if _bsuccess
        (Variables|Default|SetCurrentResourcesRate (Variables|/Game/HexRTS/Blueprints/Managers/RTSGameMode.RTSGameMode_C|GetResourcesDefault _asrtsgame_mode))
        ;[1 1 1] Add self to resources set
        (Utilities|Map|Add _resourcesperplayer (Utilities|Map|Length _resourcesperplayer) self)))))

(fn ConstructionScript)