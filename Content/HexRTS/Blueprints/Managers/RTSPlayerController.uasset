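; Player controller for the hex RTS that creates the player HUD and relays player actions to the game mode and game state.
; Server events forward objective and resource captures and hexagon terraforming.
; Unit upgrades price changed units from DT_Units, check resources locally, then route to the server, which rechecks, charges and multicasts the Polyform transformation.
; An authority-only key spawns a unit above the cursor hit point.
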(event Custom|Server_CaptureResources
  (params (ResourcesID :type Integer))
  ;[1 1 1] Capture Resources
  (Default|ServerPlayerCapturedResource (.AsRTSGame%20Mode (Utilities|Casting|CastToRTSGameMode (Game|GetGameMode))) (Variables|Network|GetID) ResourcesID))

(event Custom|Server_UpdateUnits
  (params (SelectedUnits :type Array%20of%20BP%20Unit%20Object%20References) (EndUnit :type Units%20Structure) (PlayerID :type Integer))
  ;[1 1 1] UpdateUnits
  (CallFunction|UpdateUnits SelectedUnits EndUnit PlayerID))

(event Custom|Server_CaptureObjective
  (params (ObjectiveID :type Integer))
  ;[1 1 1] Capture Objective
  (Default|ServerPlayerCapturedObjective (.AsRTSGame%20Mode (Utilities|Casting|CastToRTSGameMode (Game|GetGameMode))) (Variables|Network|GetID) ObjectiveID))

(event Custom|Multi_DoUpdateUnits
  (params (SelectedUnits :type Array%20of%20BP%20Unit%20Object%20References) (EndUnit :type Units%20Structure))
  ;[1 1 1] UpdateUnits
  (for _array_element SelectedUnits
    (Default|Polyform _array_element (.Class (Utilities|Struct|BreakUnits EndUnit)))))

(event Custom|TryUpdateUnits
  (params (SelectedUnits :type Array%20of%20BP%20Unit%20Object%20References) (EndUnit :type Units%20Structure))
  ;[1 1 1] UpdateUnits
  (CallFunction|UpdateUnits SelectedUnits EndUnit (Variables|Network|GetID)))

(event Custom|Server_MoveHexagons
  (params (Position :type Vector) (Space :type Float%20%28single-precision%29) (Speed :type Float%20%28single-precision%29) (Radious :type Integer))
  ;[1 1 1] Terraform
  (Default|MultiMoveHexagons (.AsRTSGame%20State (Utilities|Casting|CastToRTSGameState (Game|GetGameState))) Position Space Speed Radious))

(event EventBeginPlay
  ;[1 1 1] Create player widget
  (bind _asbp_player (Utilities|Casting|CastToBP_Player (Pawn|GetControlledPawn)))
  (bind _returnvalue (UserInterface|CreateWidget "/Game/HexRTS/HUD/BP_Player_Widget.BP_Player_Widget_C" self _asbp_player))
  (UserInterface|Viewport|AddtoViewport _returnvalue 0)
  (bind _output_get (Variables|/Game/HexRTS/Blueprints/Characters/BP_Player.BP_Player_C|SetWidget _asbp_player _returnvalue))
  (Utilities|FlowControl|Delay 1.0)
  (bind _asrtsplayer_state (Utilities|Casting|CastToRTSPlayerState (Variables|GetPlayerState)))
  (Variables|/Game/HexRTS/HUD/BP_Player_Widget.BP_Player_Widget_C|SetplayerState _output_get _asrtsplayer_state)
  (Input|SetInputModeGameandUI self _output_get "LockAlways" false)
  (Variables|Default|SetbShowMouseCursor true))

(event Input|KeyboardEvents|Ñ
  (params (Key :type Key%20Structure))
  (bind _hitresult (Game|Player|GetHitResultUnderCursorbyChannel "TraceTypeQuery1" true))
  (bind _impactpoint (Collision|BreakHitResult _hitresult))
  (bind (_x _y _z) (Math|Vector|BreakVector _impactpoint))
  (:Pressed
    (Networking|SwitchHasAuthority
      (:Authority
        (bind _asrtsgame_mode (Utilities|Casting|CastToRTSGameMode (Game|GetGameMode)))
        (Default|ServerCreateUnit _asrtsgame_mode (Math|Vector|MakeVector _x _y (+ _z 1e+02)))))))

(fn ConstructionScript)

(fn UpdateUnits
  (params (Units :type Array%20of%20BP%20Unit%20Object%20References) (EndUnit :type Units%20Structure) (PlayerID :type Integer))
  (bind _class (Utilities|Struct|BreakUnits EndUnit))
  (bind _playerstate (Variables|GetPlayerState))
  (bind (_asrtsplayer_state _bsuccess) (Utilities|Casting|CastToRTSPlayerState _playerstate))
  ;[1 1 1] Get total cost
  (LocalVariables|SettotalUnitCost 0)
  (for _array_element Units
    (if (Utilities|Enum|NotEqual(Enum) (Variables|/Game/HexRTS/Blueprints/Units/BP_Unit.BP_Unit_C|GetCurrentUnit _array_element) _class)
      (bind _returnvalue (Utilities|GetDataTableRow "/Game/HexRTS/DataSets/DT_Units.DT_Units" (Utilities|String|StringToName (Utilities|String|EnumtoString _class)))
        (:then
          (LocalVariables|SettotalUnitCost (+ (LocalVariables|GettotalUnitCost) (.cost (Utilities|Struct|BreakUnits _returnvalue))))))))
  ;[1 1 1] Check if the player has money
  (if _bsuccess
    (if (<= (LocalVariables|GettotalUnitCost) (Variables|/Game/HexRTS/Blueprints/Managers/RTSPlayerState.RTSPlayerState_C|GetCurrentResources _asrtsplayer_state))
      (Networking|SwitchHasAuthority
        (:Authority
          ;[1 1 1] On server, subtract resources, then tell clients to transform units
          (Default|PayforUnits (.AsRTSGame%20State (Utilities|Casting|CastToRTSGameState (Game|GetGameState))) PlayerID (LocalVariables|GettotalUnitCost))
          (CallFunction|MultiDoUpdateUnits Units EndUnit))
        (:Remote
          ;;[1 1 1] If everything OK, tell server to do it
          (CallFunction|ServerUpdateUnits Units EndUnit PlayerID))))
    (else
      (Development|PrintString "ERROR: No player state" true true "(R=1.000000,G=0.045801,B=0.000000,A=1.000000)"))))