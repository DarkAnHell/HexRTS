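; Unit information actor for the HexRTS game that sets up a unit's weapon visuals and deals its attack damage.
; The construction script picks a random static mesh for the left and right weapon components from their arrays, skipping empty arrays.
; Attack applies the Damage value to a target and credits the parent actor as damage causer, which suggests use as a child actor.
; The event graph has no logic.
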(event EventBeginPlay)

(event Collision|EventActorBeginOverlap
  (params (OtherActor :type Actor%20Object%20Reference)))

(event EventTick
  (params (DeltaSeconds :type Float%20%28single-precision%29)))

(event Game|Damage|EventAnyDamage
  (params (Damage :type Float%20%28single-precision%29) (DamageType :type Damage%20Type%20Object%20Reference) (InstigatedBy :type Controller%20Object%20Reference) (DamageCauser :type Actor%20Object%20Reference)))

(fn ConstructionScript
  (bind _left_weapons (Variables|Components|GetLeft_Weapons))
  (bind _right_weapons (Variables|Components|GetRight_Weapons))
  (bind _returnvalue (Utilities|Array|Length _right_weapons))
  (bind _returnvalue_2 (Utilities|Array|Length _left_weapons))
  (if (> _returnvalue_2 0)
    (Components|StaticMesh|SetStaticMesh (Variables|Default|GetLeftWeapon) (Utilities|Array|Get(acopy) _left_weapons (Math|Random|RandomIntegerinRange 0 (- _returnvalue_2 1)))))
  (if (> _returnvalue 0)
    (Components|StaticMesh|SetStaticMesh (Variables|Default|GetRightWeapon) (Utilities|Array|Get(acopy) _right_weapons (Math|Random|RandomIntegerinRange 0 (- _returnvalue 1))))))

(fn Attack
  (params (Objetive :type BP%20Unit%20Object%20Reference))
  (bind _returnvalue (Game|Damage|ApplyDamage Objetive (Math|Conversions|ToFloat(Integer) (Variables|Attribute|GetDamage)) 0 (Actor|GetParentActor)))
  (return _returnvalue))