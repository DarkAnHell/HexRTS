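; BP_UnitFollow is a sprite actor that represents a unit on the minimap, tied to that unit through UnitRef.
; On BeginPlay it adds itself to the ShowOnlyActors list of the first BP_Minimap's scene capture and tints its Paper sprite dark blue or dark red for player 0 or 1.
; It binds to the unit's OnDestroyed event and destroys itself when the unit is destroyed.
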(event Custom|OnDestroyed_Event_0
  (params (DestroyedActor :type Actor%20Object%20Reference))
  (Actor|DestroyActor))

(event EventBeginPlay
  (bind _papersprite (Variables|Default|GetPaperSprite))
  (Game|AssignOnDestroyed (Variables|Default|Getunit_ref) (delegate Custom|OnDestroyed_Event_0))
  (bind _outactors (Actor|GetAllActorsOfClass "/Game/HexRTS/HUD/BP_Minimap.BP_Minimap_C"))
  (Utilities|Array|Add (Variables|/Script/Engine.SceneCaptureComponent|GetShowOnlyActors (Variables|/Script/Engine.SceneCapture2D|GetCaptureComponent2D (Utilities|Array|Get(acopy) _outactors))) self)
  (switch int (Variables|/Game/HexRTS/Blueprints/Units/BP_Unit.BP_Unit_C|GetPlayer (Variables|Default|Getunit_ref))
    (:0
      (Sprite|SetSpriteColor _papersprite "(R=0.000000,G=0.008203,B=0.179167,A=1.000000)"))
    (:1
      (Sprite|SetSpriteColor _papersprite "(R=0.225000,G=0.000000,B=0.008939,A=1.000000)"))))

(event Collision|EventActorBeginOverlap
  (params (OtherActor :type Actor%20Object%20Reference)))

(event EventTick
  (params (DeltaSeconds :type Float%20%28single-precision%29)))

(fn ConstructionScript)