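; Hex-map RTS unit character that transforms ("polyforms") between unit types, delegating attacks to its active form.
; Spawns PolyformCircle's forms as child actors, then swaps visibility and animation class after a transition delay.
; Move orders pass through Server/Multi events into AI Blackboard state and target-hex keys.
; Also finds its starting hex, spawns an elevated minimap icon actor, and computes ballistic launches for jumps.
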(event Custom|Multi_Move
  (params (Hexagon :type Vector) (Acceptable%20distance :type Integer))
  ;[1 1 1] Move unit
  (CallFunction|Move Hexagon Acceptable%20distance))

(event Custom|Server_Move
  (params (Hexagon :type Vector) (Acceptable%20distance :type Integer))
  ;[1 1 1] Move unit
  (CallFunction|MultiMove Hexagon Acceptable%20distance))

(event Custom|StartPolyform
  (params (ToPolyform :type BP%20Unit%20Information%20Object%20Reference) (Time :type Float%20%28single-precision%29))
  (Variables|Default|SetState "NewEnumerator3")
  (Utilities|FlowControl|Delay Time)
  (Rendering|SetActorHiddenInGame (Variables|Default|GetCurrentUnitClass) true)
  (Components|SkeletalMesh|SetAnimInstanceClass (Variables|/Game/HexRTS/Blueprints/Units/BP_UnitInformation.BP_UnitInformation_C|GetSkeletalMesh (Variables|Default|GetCurrentUnitClass)) 0)
  (bind _output_get (Variables|Default|SetCurrentUnitClass ToPolyform))
  (Rendering|SetActorHiddenInGame _output_get false)
  (Components|SkeletalMesh|SetAnimInstanceClass (Variables|/Game/HexRTS/Blueprints/Units/BP_UnitInformation.BP_UnitInformation_C|GetSkeletalMesh (Variables|Default|GetCurrentUnitClass)) (Variables|/Game/HexRTS/Blueprints/Units/BP_UnitInformation.BP_UnitInformation_C|GetAnimationBlueprint (Variables|Default|GetCurrentUnitClass)))
  (Variables|Default|SetCurrentUnit (Variables|/Game/HexRTS/Blueprints/Units/BP_UnitInformation.BP_UnitInformation_C|GetUnitType (Variables|Default|GetCurrentUnitClass)))
  (Variables|Default|SetState "NewEnumerator0"))

(event EventBeginPlay
  (bind _returnvalue (Transformation|GetActorLocation))
  (bind (_x _y) (Math|Vector|BreakVector _returnvalue))
  (bind _returnvalue_2 (Game|SpawnActorfromClass "/Game/HexRTS/Blueprints/Units/unitFollow.unitFollow_C" (Math|Transform|MakeTransform (Math|Vector|MakeVector _x _y 1e+04)) "Undefined" 0 self 0))
  (Variables|Default|SetminimapIcon_ref _returnvalue_2)
  (bind _polyformations (CallFunction|CreatePolyform))
  (Variables|Default|SetPolyformations _polyformations)
  (bind _outactors (Actor|GetAllActorsOfClass "/Game/HexRTS/Blueprints/GridAndHexagons/BP_HexagonMapManager.BP_HexagonMapManager_C"))
  (Variables|/Script/HexRTS.PathFinding|SetMap (Variables|Default|GetPathFinding) (Utilities|Array|Get(acopy) _outactors))
  (bind _array_element (Utilities|Array|ForEachLoopwithBreak (Variables|Default|GetPolyformations) :!label _label)
    (:LoopBody
      (if (Utilities|Enum|Equal(Enum) (Variables|/Game/HexRTS/Blueprints/Units/BP_UnitInformation.BP_UnitInformation_C|GetUnitType _array_element) (Variables|Default|GetCurrentUnit))
        (Variables|Default|SetCurrentUnitClass _array_element)
        (goto _label Break)))
    (:Completed
      (CallFunction|Polyform "NewEnumerator0")
      (bind _returnvalue_3 (Class|HexagonMapManager|GetHexagon (Variables|/Script/HexRTS.PathFinding|GetMap (Variables|Default|GetPathFinding)) (Transformation|GetActorLocation)))
      (Variables|Default|SetPosition _returnvalue_3))))

(fn ConstructionScript)

(fn CreatePolyform
  (bind _polyformcircle (Variables|Default|GetPolyformCircle))
  (for _array_element (Variables|/Game/HexRTS/Blueprints/Units/Components/PolyformCircle.PolyformCircle_C|GetSpetialUnits _polyformcircle)
    (LocalVariables|Setclass _array_element)
    (bind _returnvalue (AddComponent|AddChildActorComponent false (Transformation|GetRelativeTransform (Variables|Character|GetMesh))))
    (ChildActorComponent|SetChildActorClass _returnvalue (LocalVariables|Getclass)))
  (for _array_element_2 (Variables|/Game/HexRTS/Blueprints/Units/Components/PolyformCircle.PolyformCircle_C|GetUnits _polyformcircle)
    (LocalVariables|Setclass _array_element_2)
    (bind _returnvalue_2 (AddComponent|AddChildActorComponent false (Transformation|GetRelativeTransform (Variables|Character|GetMesh))))
    (ChildActorComponent|SetChildActorClass _returnvalue_2 (LocalVariables|Getclass)))
  (for _array_element_3 (Actor|GetAllChildActors true)
    (bind _asbp_unit_information (Utilities|Casting|CastToBP_UnitInformation _array_element_3))
    (Utilities|Array|Add (LocalVariables|GetPolyfor) _asbp_unit_information))
  (return (LocalVariables|GetPolyfor)))

(fn Polyform
  (params (Polyform :type Units%20Enum :default "NewEnumerator0"))
  (bind _array_element (Utilities|Array|ForEachLoopwithBreak (Variables|Default|GetPolyformations) :!label _label)
    (:LoopBody
      (if (== (Variables|/Game/HexRTS/Blueprints/Units/BP_UnitInformation.BP_UnitInformation_C|GetUnitType _array_element) Polyform)
        (LocalVariables|SetToPolyform _array_element)
        (goto _label Break)))
    (:Completed
      (bind _time (Default|GetTimetoPolyform (Variables|Default|GetPolyformCircle) (Utilities|GetClass (Variables|Default|GetCurrentUnitClass)) (Utilities|GetClass (LocalVariables|GetToPolyform))))
      (CallFunction|StartPolyform (LocalVariables|GetToPolyform) (Math|Conversions|ToFloat(Integer) _time)))))

(fn Move
  (params (Hexagon :type Vector) (AceptableDistance :type Integer))
  (bind _returnvalue (Pawn|GetController))
  (bind _returnvalue_2 (AI|GetBlackboard _returnvalue))
  (bind _output_get (Variables|Default|SetState "NewEnumerator0"))
  (AI|Components|Blackboard|SetValueasEnum _returnvalue_2 (Variables|Keys|GetStateKeyName) _output_get)
  (AI|Components|Blackboard|SetValueasVector _returnvalue_2 (Variables|Keys|GetHexagonPositionKeyName) Hexagon)
  (bind _output_get_2 (Variables|Default|SetState "NewEnumerator1"))
  (AI|Components|Blackboard|SetValueasEnum _returnvalue_2 (Variables|Keys|GetStateKeyName) _output_get_2))

(fn JumptoPoint
  (params (Point :type Vector))
  (bind _currentunitclass (Variables|Default|GetCurrentUnitClass))
  (bind _movementspeed (Variables|/Game/HexRTS/Blueprints/Units/BP_UnitInformation.BP_UnitInformation_C|GetMovementSpeed _currentunitclass))
  (LocalVariables|SetVx (Math|Conversions|ToFloat(Integer) _movementspeed))
  (bind _output_get (LocalVariables|SetT (/ (Math|Vector|VectorLengthXY (- Point (Transformation|GetActorLocation))) (Math|Conversions|ToFloat(Integer) _movementspeed))))
  (bind _output_get_2 (LocalVariables|SetVy (/ (+ (/ (* (Math|Float|Power _output_get 2.0) (Math|Float|Absolute(Float) (Components|Movement|GetGravityZ (Variables|Character|GetCharacterMovement)))) 2.0) (- (.Z (Math|Vector|BreakVector "0, 0, 0")) (- (.z (Transformation|GetActorLocation)) (- (Components|Capsule|GetScaledCapsuleHalfHeight (Variables|Collision|GetCapsuleComponent)) 13.0)))) _output_get)))
  (Character|LaunchCharacter (Math|Vector|RotateVector (Math|Vector|MakeVector 0.0 (LocalVariables|GetVx) (LocalVariables|GetVy)) (Math|Rotator|FindLookatRotation (Math|Vector|MakeVector 0.0 (LocalVariables|GetVx) (LocalVariables|GetVy)) (Transformation|GetActorForwardVector))) false false)
  (Development|PrintString (Utilities|String|ToString(Vector) (Math|Vector|MakeVector 0.0 (LocalVariables|GetVx) (LocalVariables|GetVy)))))

(fn Attack
  (Default|Attack (Variables|Default|GetCurrentUnitClass) (Variables|Default|GetObjective)))

(fn UpdateIconPosition
  (bind _returnvalue (Transformation|GetActorLocation))
  (bind _minimapicon_ref (Variables|Default|GetminimapIcon_ref))
  (bind (_x _y) (Math|Vector|BreakVector _returnvalue))
  (Transformation|SetActorLocation _minimapicon_ref (Math|Vector|MakeVector _x _y (.Z (Math|Vector|BreakVector (Transformation|GetActorLocation _minimapicon_ref)))) false false))