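; BP_ResourcePoints is a capturable resource point for an RTS, claimed by players' units.
; Each tick it checks units overlapping its sphere, resetting progress when players conflict and transferring ownership to the provisional army once the conquest timer expires.
; CheckConection maintains links between a conquered point and nearby points using height-offset line traces, but nothing here calls it.
; SearchForPath, meant to run toward a base when links change, is an empty loop.
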(event EventBeginPlay)

(event Collision|EventActorBeginOverlap
  (params (OtherActor :type Actor%20Object%20Reference)))

(event EventTick
  (params (DeltaSeconds :type Float%20%28single-precision%29))
  (CallFunction|StartConquestPoint))

(fn ConstructionScript)

(fn StartConquestPoint
  (bind _array_element (Utilities|Array|ForEachLoopwithBreak (Collision|GetOverlappingActors (Variables|Default|GetSphere) "/Game/HexRTS/Units/Unit.Unit_C" :!class /Script/Engine.PrimitiveComponent) :!label _label)
    (:LoopBody
      (bind _asunit (Utilities|Casting|CastToUnit _array_element))
      (if (== (Variables|Conquest|GetProvArmy) 0)
        (Variables|Conquest|SetProvArmy (Variables|/Game/HexRTS/Units/Unit.Unit_C|GetPlayer _asunit))
        (Variables|Conquest|SetStartConquest true)
        (elif (!= (Variables|Conquest|GetProvArmy) (Variables|/Game/HexRTS/Units/Unit.Unit_C|GetPlayer _asunit))
          (Variables|Conquest|SetStartConquest false)
          (Variables|Conquest|SetProvArmy 0)
          (Variables|Conquest|SetTime 0.0)
          (goto _label Break))))
    (:Completed
      (if (Variables|Conquest|GetStartConquest)
        (if (!= (Variables|Conquest|GetProvArmy) (Variables|Conquest|GetConquerArmy))
          (bind _output_get (Variables|Conquest|SetTime (+ (Variables|Conquest|GetTime) (Utilities|Time|GetWorldDeltaSeconds))))
          (if (> _output_get (Variables|Conquest|GetConquestTime))
            (Variables|Conquest|SetConquerArmy (Variables|Conquest|GetProvArmy))
            (Variables|Conquest|SetStartConquest false)
            (Variables|Conquest|SetIsConquest true)))))))

(fn CheckConection
  (bind _returnvalue (Transformation|GetActorLocation))
  (bind _raycastmargin (Variables|Connection|GetRaycastMargin))
  (bind _connectedpoints (Variables|Connection|GetConnectedPoints))
  (bind _connectedpoints_2 (Variables|Connection|GetConnectedPoints))
  (bind (_x _y _z) (Math|Vector|BreakVector _returnvalue))
  (bind _returnvalue_2 (+ _z _raycastmargin))
  (if (Variables|Conquest|GetIsConquest)
    (for _array_element (Variables|Connection|GetNearPoints)
      (bind _outhit (Collision|LineTraceByChannel (Math|Vector|MakeVector _x _y _returnvalue_2) (Math|Vector|MakeVector (.X (Math|Vector|BreakVector (Transformation|GetActorLocation _array_element))) (.Y (Math|Vector|BreakVector (Transformation|GetActorLocation _array_element))) _returnvalue_2) "TraceTypeQuery1" false 0 "ForOneFrame"))
      (Utilities|Casting|CastToBP_ResourcePoints (.HitActor (Collision|BreakHitResult _outhit))
        (:then
          (if (not (Utilities|Array|ContainsItem _connectedpoints_2 _array_element))
            (Utilities|Array|Add _connectedpoints_2 _array_element)
            (if (== (Utilities|Array|Length _connectedpoints_2) 0) :!label _label
              (Variables|Connection|SetIsConnected false)
              (else
                (CallFunction|SearchforPath (Variables|Default|GetBaseRef))))))
        (:CastFailed
          (if (Utilities|Array|ContainsItem _connectedpoints _array_element)
            (Utilities|Array|RemoveItem _connectedpoints _array_element)
            (goto _label)))))))

(fn SearchforPath
  (params (Base :type BP%20Resource%20Points%20Object%20Reference))
  (for _array_element (Variables|Connection|GetConnectedPoints)
    _))