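; BP_MenuPlayer is the menu player actor that publishes a player's ID and name to the lobby UI.
; One second after BeginPlay, it reads the ID from player controller 0's BP_MenuController and the name from RTSGameInstance.
; It passes them through a server event to a multicast event, which calls SetPlayerData on the first BP_Lobby_Widget found, if valid.
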(event Custom|Server_SetLobby
  (params (ID :type Integer) (Name :type String))
  (CallFunction|MultiUpdateLobby ID Name))

(event Custom|Multi_UpdateLobby
  (params (ID :type Integer) (Name :type String))
  (bind _foundwidgets (Widget|GetAllWidgetsOfClass "/Game/HexRTS/HUD/BP_Lobby_Widget.BP_Lobby_Widget_C" false))
  (Utilities|IsValid (Utilities|Array|Get(acopy) _foundwidgets)
    (:Is%20Valid
      (Default|SetPlayerData (Utilities|Array|Get(acopy) _foundwidgets) ID Name))))

(event EventBeginPlay
  (Utilities|FlowControl|Delay 1.0)
  (CallFunction|ServerSetLobby (Variables|/Game/HexRTS/Blueprints/Characters/BP_MenuController.BP_MenuController_C|GetID (.AsBP%20Menu%20Controller (Utilities|Casting|CastToBP_MenuController (Game|GetPlayerController 0)))) (Variables|/Game/HexRTS/Blueprints/Managers/RTSGameInstance.RTSGameInstance_C|GetPlayerName (.AsRTSGame%20Instance (Utilities|Casting|CastToRTSGameInstance (Game|GetGameInstance))))))

(fn ConstructionScript)