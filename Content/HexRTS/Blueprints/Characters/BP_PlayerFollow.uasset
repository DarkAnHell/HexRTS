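; BP_PlayerFollow is an actor that shadows the player high above the world and appears in the minimap capture.
; On BeginPlay it adds itself to the ShowOnlyActors list of the first BP_Minimap's CaptureComponent2D.
; Each Tick it copies PlayerRef's X, Y and yaw while holding a fixed height, with pitch and roll zeroed.
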(event EventBeginPlay
  (bind _outactors (Actor|GetAllActorsOfClass "/Game/HexRTS/HUD/BP_Minimap.BP_Minimap_C"))
  (Utilities|Array|Add (Variables|/Script/Engine.SceneCaptureComponent|GetShowOnlyActors (Variables|/Script/Engine.SceneCapture2D|GetCaptureComponent2D (Utilities|Array|Get(acopy) _outactors))) self))

(event Collision|EventActorBeginOverlap
  (params (OtherActor :type Actor%20Object%20Reference)))

(event EventTick
  (params (DeltaSeconds :type Float%20%28single-precision%29))
  (bind _player_ref (Variables|Default|GetPlayer_ref))
  (bind _returnvalue (Transformation|GetActorTransform _player_ref))
  (bind (_location _rotation) (Math|Transform|BreakTransform _returnvalue))
  (bind (_x _y) (Math|Vector|BreakVector _location))
  (Transformation|SetActorLocationAndRotation (Math|Vector|MakeVector _x _y 2e+04) (Math|Rotator|MakeRotator 0.0 0.0 (.Yaw (Math|Rotator|BreakRotator _rotation)))))

(fn ConstructionScript)