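; BP_SelectorBox is an actor that displays a rectangular area, apparently the mouse-drag selection box for the RTS.
; DrawArea converts a given world position into the root's local space, then moves the visual area parent to the midpoint between root and that point.
; It scales that component's X and Y by the absolute half-offsets divided by MouseDragMargin, keeping Z thin.
; The event graph and construction script are empty.
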(event EventBeginPlay)

(event Collision|EventActorBeginOverlap
  (params (OtherActor :type Actor%20Object%20Reference)))

(event EventTick
  (params (DeltaSeconds :type Float%20%28single-precision%29)))

(fn ConstructionScript)

(fn DrawArea
  (params (Pos :type Vector))
  (bind _mousedragmargin (Variables|Default|GetMouseDragMargin))
  (bind _visalareaparent (Variables|Default|GetVisalAreaParent))
  (Variables|Default|SetPosition (Math|Transform|InverseTransformLocation (Transformation|GetWorldTransform (Variables|Default|GetDefaultSceneRoot)) Pos))
  (Transformation|SetRelativeLocation _visalareaparent (/ (Variables|Default|GetPosition) 2.0) false false)
  (Transformation|SetRelativeScale3D _visalareaparent (Math|Vector|MakeVector (Math|Float|Absolute(Float) (/ (.X (Math|Vector|BreakVector (/ (Variables|Default|GetPosition) 2.0))) _mousedragmargin)) (Math|Float|Absolute(Float) (/ (.Y (Math|Vector|BreakVector (/ (Variables|Default|GetPosition) 2.0))) _mousedragmargin)) 0.05)))