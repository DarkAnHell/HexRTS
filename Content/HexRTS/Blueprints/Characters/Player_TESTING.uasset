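; Test RTS camera player for HexRTS that pans and zooms along the camera view and shows the mouse cursor.
; Axis inputs move the actor by local offsets, with zoom gated by a height range that only permits reversing once outside it.
; N and M keys call the game instance to join or host a LAN game.
; Edge scrolling is never run, and unit selection is mostly stubbed.
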(event EventBeginPlay
  (Variables|/Script/Engine.PlayerController|SetbShowMouseCursor (Game|GetPlayerController 0) true))

(event EventTick
  (params (DeltaSeconds :type Float%20%28single-precision%29))
  ;[1 1 1] Mouse: movement
)

(event Collision|EventActorEndOverlap
  (params (OtherActor :type Actor%20Object%20Reference)))

(event Input|ActionEvents|InputActionClick
  (params (Key :type Key%20Structure))
  (:Pressed
    (Variables|Selection|SetIsSelected true))
  (:Released
    (Variables|Selection|SetIsSelected false)
    (Utilities|IsValid (Variables|Selection|GetSelectionBox)
      (:Is%20Valid
        (CallFunction|AddSelectedUnits))
      (:Is%20Not%20Valid
        (Utilities|Casting|CastToUnit (stale Collision|EventActorEndOverlap OtherActor)
          (:CastFailed
            (if (> (Utilities|Array|Length (Variables|Selection|GetSelectedMinions)) 0)
              _)))))))

(event Input|AxisEvents|InputAxisMoveForward
  (params (AxisValue :type Float%20%28single-precision%29))
  ;[1 1 1] Keys movement
  (CallFunction|MoveForward AxisValue))

(event Input|AxisEvents|InputAxisMoveZoom
  (params (AxisValue :type Float%20%28single-precision%29))
  ;[1 1 1] Keys zoom
  (CallFunction|MoveZoom AxisValue))

(event Input|AxisEvents|InputAxisMoveRight
  (params (AxisValue :type Float%20%28single-precision%29))
  ;[1 1 1] Keys movement
  (CallFunction|MoveRight AxisValue))

(event Input|KeyboardEvents|M
  (params (Key :type Key%20Structure))
  (:Released
    (Development|PrintString "BABY")
    (bind _asrtsgame_instance (Utilities|Casting|CastToRTSGameInstance (Game|GetGameInstance))
      (:then
        (Default|ServerHostGame _asrtsgame_instance true (Game|GetPlayerController 0) 2))
      (:CastFailed
        (Development|PrintString "NOT EVEN CLOSE")))))

(event Input|KeyboardEvents|N
  (params (Key :type Key%20Structure))
  (:Released
    (Development|PrintString "NNNN")
    (bind _asrtsgame_instance (Utilities|Casting|CastToRTSGameInstance (Game|GetGameInstance))
      (:then
        (Default|ServerJoinGame _asrtsgame_instance (Game|GetPlayerController 0) true))
      (:CastFailed
        (Development|PrintString "Nah man")))))

(fn ConstructionScript)

(fn MoveForward
  (params (Axis :type Float%20%28single-precision%29))
  (Transformation|AddActorLocalOffset (Math|Vector|MakeVector (* Axis (Utilities|Time|GetWorldDeltaSeconds) (Variables|Move|GetMovSpeed)) 0.0 0.0) true false))

(fn MoveRight
  (params (Axis :type Float%20%28single-precision%29))
  (Transformation|AddActorLocalOffset (Math|Vector|MakeVector 0.0 (* Axis (Utilities|Time|GetWorldDeltaSeconds) (Variables|Move|GetMovSpeed)) 0.0) true false))

(fn MoveZoom
  (params (Axis :type Float%20%28single-precision%29))
  (bind _canzoom (CallFunction|ZoomRange Axis))
  (if _canzoom
    (Transformation|AddActorLocalOffset (* (Math|Vector|GetForwardVector (Variables|Default|GetPlayerCamera)) (* Axis (Utilities|Time|GetWorldDeltaSeconds) (Variables|Move|GetZoomSpeed))) false false)))

(fn CheckMousePosition
  (bind _returnvalue (Viewport|GetViewportSize))
  (bind _returnvalue_2 (Game|GetPlayerController 0))
  (bind _mousemargin (Variables|Move|GetMouseMargin))
  (bind _mousemargin_2 (Variables|Move|GetMouseMargin))
  (bind (_x _y) (Math|Vector2D|BreakVector2D _returnvalue))
  (bind (_locationx _locationy) (Game|Player|GetMousePosition _returnvalue_2))
  (if (< (- _x _mousemargin) _locationx)
    (CallFunction|MoveRight 1.0)
    (elif (> _mousemargin _locationx)
      (CallFunction|MoveRight -1.0)))
  (if (< (- _y _mousemargin_2) _locationy)
    (CallFunction|MoveForward -1.0)
    (elif (> _mousemargin_2 _locationy)
      (CallFunction|MoveForward 1.0))))

(fn ZoomRange
  (params (Axis :type Float%20%28single-precision%29))
  (bind _returnvalue (Transformation|GetActorLocation))
  (bind _z (Math|Vector|BreakVector _returnvalue))
  (if (and (>= (Variables|Move|GetMaxHeight) _z) (<= (Variables|Move|GetMinHeight) _z))
    (Variables|Move|SetPreviewsAxis Axis)
    (elif (< (Variables|Move|GetPreviewsAxis) 0.0)
      (if (>= Axis 0.0)
        _
        (else
          (return false)))
      (elif (<= Axis 0.0)
        _
        (else
          (return false)))))
  (return true))

(fn AddSelectedUnits)

(fn EmptyList
  (bind _selectedminions (Variables|Selection|GetSelectedMinions))
  (for _array_element _selectedminions
    _)
  (Utilities|Array|Clear _selectedminions))

(fn Selection)