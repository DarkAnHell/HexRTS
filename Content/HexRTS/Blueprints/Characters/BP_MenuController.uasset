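; Menu player controller for HexRTS that shows the mouse cursor and handles hosting and joining multiplayer sessions.
; Hosting creates a session with the given LAN and connection-count settings, then opens the Lobby level as a listen server.
; Joining searches for sessions and calls JoinSession on every result rather than selecting one.
; Failed session creation or search prints red error text.
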(event Custom|Server_HostGame
  (params (UseLAN? :type Boolean) (Public%20Connections :type Integer))
  ;[0.5986 0.3972 1] Session Management
  ;;[1 1 1] Host game
  (|Session self Public%20Connections UseLAN?
    (:OnSuccess
      (Game|OpenLevel(byName) "Lobby" true "listen"))
    (:OnFailure
      (Development|PrintText "Error when creating a session" true true "(R=1.000000,G=0.000000,B=0.064177,A=1.000000)"))))

(event Custom|Server_JoinGame
  (params (Use%20LAN :type Boolean))
  (bind _self self)
  ;[0.5986 0.3972 1] Session Management
  ;;[1 1 1] Join Game
  (bind _results (|FindSessions _self 10 Use%20LAN)
    (:OnSuccess
      (for _array_element _results
        (|JoinSession _self _array_element)))
    (:OnFailure
      (Development|PrintText "Failed to find a session" true true "(R=1.000000,G=0.000000,B=0.019289,A=1.000000)"))))

(event EventBeginPlay
  (Variables|Default|SetbShowMouseCursor true))

(fn ConstructionScript)