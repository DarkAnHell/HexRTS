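; BP_Arrow is an arrow projectile for the HexRTS game that turns on Tick to follow its velocity.
; CalculeForce returns a ballistic launch velocity toward a target position, solved from projectile gravity and height difference.
; Flight time is FlyTime multiplied by the horizontal distance in rounded-up steps of four times the hex map manager's ScaleXY.
; The horizontal heading comes from a doubled look-at yaw between normalized vectors.
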(event EventBeginPlay)

(event Collision|EventActorBeginOverlap
  (params (OtherActor :type Actor%20Object%20Reference)))

(event EventTick
  (params (DeltaSeconds :type Float%20%28single-precision%29))
  (Transformation|SetActorRotation (Math|Rotator|FindLookatRotation (Math|Vector|GetForwardVector (Variables|Default|GetDefaultSceneRoot)) (Transformation|GetVelocity))))

(fn ConstructionScript)

(fn CalculeForce
  (params (Position :type Vector))
  (bind _outactors (Actor|GetAllActorsOfClass "/Game/HexRTS/Blueprints/GridAndHexagons/BP_HexagonMapManager.BP_HexagonMapManager_C"))
  (Variables|Default|SetObjetive Position)
  (LocalVariables|SetVx (/ (Math|Vector|VectorLengthXY (- (Transformation|GetActorLocation) (Variables|Default|GetObjetive))) (* (Variables|Default|GetFlyTime) (Math|Conversions|ToFloat(Integer) (Math|Float|Ceil (/ (Math|Vector|VectorLengthXY (- (Transformation|GetActorLocation) (Variables|Default|GetObjetive))) (Math|Conversions|ToFloat(Integer) (* (Variables|/Script/HexRTS.HexagonMapManager|GetscaleXY (Utilities|Array|Get(acopy) _outactors)) 4))))))))
  (bind _output_get (LocalVariables|SetT (* (Variables|Default|GetFlyTime) (Math|Conversions|ToFloat(Integer) (Math|Float|Ceil (/ (Math|Vector|VectorLengthXY (- (Transformation|GetActorLocation) (Variables|Default|GetObjetive))) (Math|Conversions|ToFloat(Integer) (* (Variables|/Script/HexRTS.HexagonMapManager|GetscaleXY (Utilities|Array|Get(acopy) _outactors)) 4))))))))
  (LocalVariables|SetVy (/ (+ (/ (* (Math|Float|Power _output_get 2.0) (Math|Float|Absolute(Float) (Components|Movement|GetGravityZ (Variables|Default|GetProjectileMovement)))) 2.0) (- (.Z (Math|Vector|BreakVector (Variables|Default|GetObjetive))) (.z (Transformation|GetActorLocation)))) _output_get))
  (return (Math|Vector|RotateVector (Math|Vector|MakeVector 0.0 (LocalVariables|GetVx) (LocalVariables|GetVy)) (Math|Rotator|MakeRotator 0.0 0.0 (* (.Yaw (Math|Rotator|BreakRotator (Math|Rotator|FindLookatRotation (Math|Vector|Normalize (Math|Vector|MakeVector (.x (Variables|Default|GetObjetive)) (.y (Variables|Default|GetObjetive)) 0.0)) (Math|Vector|Normalize (Math|Vector|MakeVector 0.0 (LocalVariables|GetVx) 0.0))))) 2.0)))))