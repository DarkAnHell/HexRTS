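; Hex-map RTS unit character that can switch between the unit forms listed in its polyform circle.
; It spawns each form as a child actor, then Polyform copies the selected form's skeletal mesh and animation class.
; Move requests a hex path, feeding waypoints one by one to the AI blackboard as MoveComplete fires.
; JumpToPoint derives a ballistic launch velocity from movement speed, distance and gravity.
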(event Custom|MoveComplete
  (bind _path (Variables|Default|GetPath))
  (if (> (Utilities|Array|Length _path) 0)
    (CallFunction|SimpleMove (.pos (Utilities|Struct|BreakhexagInfo (Utilities|Array|Get(acopy) _path))))
    (Utilities|Array|RemoveIndex _path)))

(event EventBeginPlay
  (bind _polyformations (CallFunction|CreatePolyform))
  (Variables|Default|SetPolyformations _polyformations)
  (bind _outactors (Actor|GetAllActorsOfClass "/Game/HexRTS/Blueprints/GridAndHexagons/BP_HexagonMapManager.BP_HexagonMapManager_C"))
  (Variables|/Script/HexRTS.PathFinding|SetMap (Variables|Default|GetPathFinding) (Utilities|Array|Get(acopy) _outactors))
  (CallFunction|Polyform "NewEnumerator1"))

(event Collision|EventActorBeginOverlap
  (params (OtherActor :type Actor%20Object%20Reference)))

(event EventTick
  (params (DeltaSeconds :type Float%20%28single-precision%29)))

(fn ConstructionScript)

(fn CreatePolyform
  (bind _polyformcircle (Variables|Default|GetPolyformCircle))
  (for _array_element (Variables|/Game/HexRTS/Units/Components/PolyformCircle.PolyformCircle_C|GetSpetialUnits _polyformcircle)
    (LocalVariables|Setclass _array_element)
    (bind _returnvalue (AddComponent|AddChildActorComponent false))
    (ChildActorComponent|SetChildActorClass _returnvalue (LocalVariables|Getclass)))
  (for _array_element_2 (Variables|/Game/HexRTS/Units/Components/PolyformCircle.PolyformCircle_C|GetUnits _polyformcircle)
    (LocalVariables|Setclass _array_element_2)
    (bind _returnvalue_2 (AddComponent|AddChildActorComponent false))
    (ChildActorComponent|SetChildActorClass _returnvalue_2 (LocalVariables|Getclass)))
  (for _array_element_3 (Actor|GetAllChildActors true)
    (bind _asbp_unit_information (Utilities|Casting|CastToBP_UnitInformation _array_element_3))
    (Utilities|Array|Add (LocalVariables|GetPolyfor) _asbp_unit_information))
  (return (LocalVariables|GetPolyfor)))

(fn Polyform
  (params (Polyform :type Units%20Enum :default "NewEnumerator0"))
  (bind _array_element (Utilities|Array|ForEachLoopwithBreak (Variables|Default|GetPolyformations) :!label _label)
    (:LoopBody
      (if (== (Variables|/Game/HexRTS/Units/BP_UnitInformation.BP_UnitInformation_C|GetUnitType _array_element) Polyform)
        (LocalVariables|SetToPolyform _array_element)
        (goto _label Break)))
    (:Completed
      (Default|GetTimetoPolyform (Variables|Default|GetPolyformCircle) (Utilities|GetClass (Variables|Default|GetCurrentUnitClass)) (Utilities|GetClass (LocalVariables|GetToPolyform)))
      (bind _output_get (Variables|Default|SetCurrentUnitClass (LocalVariables|GetToPolyform)))
      (Class|SkinnedMeshComponent|SetSkeletalMesh (Variables|Character|GetMesh) (Variables|/Script/Engine.SkinnedMeshComponent|GetSkeletalMesh (Variables|/Game/HexRTS/Units/BP_UnitInformation.BP_UnitInformation_C|GetSkeletalMesh _output_get)) true)
      (Components|SkeletalMesh|SetAnimInstanceClass (Variables|Character|GetMesh) (Utilities|GetClass (Components|SkeletalMesh|GetAnimInstance (Variables|/Game/HexRTS/Units/BP_UnitInformation.BP_UnitInformation_C|GetSkeletalMesh _output_get))))
      (Variables|Default|SetCurrentUnit (Variables|/Game/HexRTS/Units/BP_UnitInformation.BP_UnitInformation_C|GetUnitType (Variables|Default|GetCurrentUnitClass))))))

(fn Move
  (params (PosVector :type Hexag%20Info%20Structure))
  (bind _output_get (Variables|Default|SetState "NewEnumerator0"))
  (AI|Components|Blackboard|SetValueasEnum (AI|GetBlackboard (Pawn|GetController)) (Variables|Keys|GetStateKeyName) _output_get)
  (bind _returnvalue (Class|HexagonMapManager|SeeAround (Variables|/Script/HexRTS.PathFinding|GetMap (Variables|Default|GetPathFinding)) (Transformation|GetActorLocation)))
  (bind _returnvalue_2 (Class|PathFinding|Pathto (Variables|Default|GetPathFinding) (Utilities|Array|Get(acopy) _returnvalue) PosVector))
  (bind _output_get_2 (Variables|Default|SetPath _returnvalue_2))
  (if (> (Utilities|Array|Length _output_get_2) 0)
    (CallFunction|SimpleMove (.pos (Utilities|Struct|BreakhexagInfo (Utilities|Array|Get(acopy) _output_get_2))))
    (Utilities|Array|RemoveIndex _output_get_2)
    (else
      (Development|PrintString "No hay path"))))

(fn JumptoPoint
  (params (Point :type Vector))
  (bind _currentunitclass (Variables|Default|GetCurrentUnitClass))
  (bind _movementspeed (Variables|/Game/HexRTS/Units/BP_UnitInformation.BP_UnitInformation_C|GetMovementSpeed _currentunitclass))
  (LocalVariables|SetVx (Math|Conversions|ToFloat(Integer) _movementspeed))
  (bind _output_get (LocalVariables|SetT (/ (Math|Vector|VectorLengthXY (- Point (Transformation|GetActorLocation))) (Math|Conversions|ToFloat(Integer) _movementspeed))))
  (bind _output_get_2 (LocalVariables|SetVy (/ (+ (/ (* (Math|Float|Power _output_get 2.0) (Math|Float|Absolute(Float) (Components|Movement|GetGravityZ (Variables|Character|GetCharacterMovement)))) 2.0) (- (.Z (Math|Vector|BreakVector Point)) (- (.z (Transformation|GetActorLocation)) (- (Components|Capsule|GetScaledCapsuleHalfHeight (Variables|Collision|GetCapsuleComponent)) 13.0)))) _output_get)))
  (Development|PrintString (Utilities|String|ToString(Float) _output_get_2))
  (Character|LaunchCharacter (Math|Vector|RotateVector (Math|Vector|MakeVector 0.0 (LocalVariables|GetVx) (LocalVariables|GetVy)) (Math|Rotator|FindLookatRotation (Math|Vector|MakeVector 0.0 (LocalVariables|GetVx) (LocalVariables|GetVy)) (Transformation|GetActorForwardVector))) false false)
  (Development|PrintString (Utilities|String|ToString(Vector) (Math|Vector|MakeVector 0.0 (LocalVariables|GetVx) (LocalVariables|GetVy)))))

(fn SimpleMove
  (params (Position :type Vector))
  (bind _returnvalue (Pawn|GetController))
  (bind _returnvalue_2 (AI|GetBlackboard _returnvalue))
  (bind _output_get (Variables|Default|SetState "NewEnumerator1"))
  (AI|Components|Blackboard|SetValueasVector _returnvalue_2 (Variables|Keys|GetHexagonPositionKeyName) Position)
  (AI|Components|Blackboard|SetValueasEnum _returnvalue_2 (Variables|Keys|GetStateKeyName) _output_get))