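; BP_Minimap is a scene capture actor that frames the hex map for the HUD minimap.
; On alternate ticks it searches for BP_HexagonMapManager until one is found, then adds its HexagonClass to the capture's ShowOnlyActors list and moves high above the map's center.
; The other ticks print the first show-only entry's name as debug output, even after setup finishes.
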(event EventTick
  (params (DeltaSeconds :type Float%20%28single-precision%29))
  (Utilities|FlowControl|FlipFlop
    (:A
      (if (not (Variables|Default|GethasFoundMap))
        (bind _outactors (Actor|GetAllActorsOfClass "/Game/HexRTS/Blueprints/GridAndHexagons/BP_HexagonMapManager.BP_HexagonMapManager_C"))
        (Utilities|IsValid (Utilities|Array|Get(acopy) _outactors)
          (:Is%20Valid
            (Variables|Default|SethasFoundMap true)
            (Utilities|Array|Add (Variables|/Script/Engine.SceneCaptureComponent|GetShowOnlyActors (Variables|DecalActor|GetCaptureComponent2D)) (Variables|/Script/HexRTS.HexagonMapManager|GethexagonClass (Utilities|Array|Get(acopy) _outactors)))
            (bind _returnvalue (Class|HexagonMapManager|GetCenter (Utilities|Array|Get(acopy) _outactors)))
            (Transformation|SetActorLocation (Math|Vector|MakeVector (.X (Math|Vector|BreakVector _returnvalue)) (.Y (Math|Vector|BreakVector _returnvalue)) 2.4e+04) false false)))))
    (:B
      (Development|PrintString (Utilities|GetDisplayName (Utilities|Array|Get(acopy) (Variables|/Script/Engine.SceneCaptureComponent|GetShowOnlyActors (Variables|DecalActor|GetCaptureComponent2D))))))))

(fn ConstructionScript)